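; BP_Rock is a rock actor that moves when something enters its Sphere trigger, then returns to its start.
; BeginPlay stores the initial location, and any Sphere overlap sets a Detection flag for five seconds.
; While the flag is set, Tick adds Dir to the location each frame, unswept and unscaled by delta time.
; Otherwise, Tick holds the rock at its initial location, so it snaps back instantly.
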(event `self.ReceiveBeginPlay`
  (set `self.initPos` (`self.K2_GetActorLocation`)))

(event `self.ReceiveTick`
  (params (DeltaSeconds :type "Float (single-precision)"))
  (if (`self.Detection`)
    (`self.K2_SetActorLocation` (+ (`self.K2_GetActorLocation`) (`self.Dir`)))
    (else
      (`self.K2_SetActorLocation` (`self.initPos`)))))

(event `self.Sphere.OnComponentBeginOverlap`
  (params (OverlappedComponent :type "PrimitiveComponent Object Reference") (OtherActor :type "Actor Object Reference") (OtherComp :type "PrimitiveComponent Object Reference") (OtherBodyIndex :type Integer) (bFromSweep :type Boolean) (SweepResult :type "HitResult Structure (by ref)"))
  (set `self.Detection` true)
  (`KismetSystemLibrary.Delay` 5.0)
  (set `self.Detection` false))

(fn `UserConstructionScript`)