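; BP_HealthUp is a health pickup that heals BP_Ninja by HealthAmount.
; When the ninja overlaps its Sphere, it sets IsEat to block repeats, plays a heal sound and particle effect, calls Heal and expires after a short lifespan.
; Tick spins the mesh, then makes it rise and spin faster once collected, using fixed per-frame steps not scaled by delta time.
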(event `self.ReceiveTick`
  (params (DeltaSeconds :type "Float (single-precision)"))
  (bind _staticmesh (`self.StaticMesh`))
  (if (not (`self.isEat`))
    (`SceneComponent.K2_AddWorldRotation` _staticmesh (struct :`Yaw` 5.0) false false)
    (else
      (`SceneComponent.K2_AddWorldTransform` _staticmesh (`KismetMathLibrary.MakeTransform` (0.0 0.0 3.0) (struct :`Yaw` 15.0) (1.0 1.0 1.0)) false false))))

(event `self.Sphere.OnComponentBeginOverlap`
  (params (OverlappedComponent :type "PrimitiveComponent Object Reference") (OtherActor :type "Actor Object Reference") (OtherComp :type "PrimitiveComponent Object Reference") (OtherBodyIndex :type Integer) (bFromSweep :type Boolean) (SweepResult :type "HitResult Structure (by ref)"))
  (bind _returnvalue (`SceneComponent.K2_GetComponentLocation` (`self.StaticMesh`)))
  (`/Engine/EditorBlueprintResources/StandardMacros.IsValid` OtherActor
    (:`Is Valid`
      (bind _asbp_ninja (cast `/Game/Models/Ninja/BP_Ninja` OtherActor))
      (if (and (== OtherActor _asbp_ninja) (not (`self.isEat`)))
        (set `self.isEat` true)
        (`GameplayStatics.PlaySoundAtLocation` "/Game/ActionAsset/Assets/Sound/Character/A_Character_Heal01.A_Character_Heal01" _returnvalue (struct) 1.0 1.0 0.0 null null null)
        (`self.SetLifeSpan` 5.0)
        (`GameplayStatics.SpawnEmitterAtLocation` "/Game/InfinityBladeEffects/Effects/FX_Monsters/FX_Monster_Ausar/P_AU_Heal_01.P_AU_Heal_01" (+ _returnvalue (0.0 0.0 200.0)))
        (`/Game/Models/Ninja/BP_Ninja.Heal` _asbp_ninja (`self.HealthAmount`))))))

(fn `UserConstructionScript`)